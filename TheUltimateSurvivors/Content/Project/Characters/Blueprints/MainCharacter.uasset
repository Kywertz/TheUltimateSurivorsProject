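; MainCharacter is the player character Blueprint, which sets up the camera and HUD and holds XP and max XP values.
; On BeginPlay it activates Camera1, then creates a WBP_HUD widget and adds it to the viewport.
; Every Tick it prints XP and MaxXp on screen as colored debug text.
; The graph only reads these values and contains no logic that changes them.
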(event EventTick
  (params (DeltaSeconds :type Float%20%28single-precision%29))
  (Development|PrintString (Utilities|String|Append "XP :" (Utilities|String|ToString(Float) (Variables|Default|GetXP))) true true "(R=1.000000,G=0.000000,B=0.102836,A=1.000000)" 0.0)
  (Development|PrintString (Utilities|String|Append "MAX XP :" (Utilities|String|ToString(Float) (Variables|Default|GetMaxXp))) true true "(R=0.000000,G=1.000000,B=0.079819,A=1.000000)" 0.0))

(event EventBeginPlay
  (Components|Activation|Activate (Variables|Default|GetCamera1) false)
  (bind _returnvalue (UserInterface|CreateWidget "/Game/Project/UI/WBP_HUD.WBP_HUD_C"))
  (UserInterface|Viewport|AddtoViewport _returnvalue 0))

(fn ConstructionScript)