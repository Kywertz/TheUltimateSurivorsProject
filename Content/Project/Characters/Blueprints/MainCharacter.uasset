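; Player character Blueprint that handles life, XP pickups, a timed attack flag and game over.
; BeginPlay creates the HUD and health widget; Tick pushes life to it, turns Widget1 toward Camera1, and at zero life disables input and shows game over.
; Capsule overlaps collect XP, LoseLife subtracts damage, and left click sets CanAttack for two seconds.
; SaveValue loads or creates MySave; overlap-based timed damage is left unwired.
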(event OnComponentBeginOverlap(CapsuleComponent)
  (params (OverlappedComponent :type Primitive%20Component%20Object%20Reference) (OtherActor :type Actor%20Object%20Reference) (OtherComp :type Primitive%20Component%20Object%20Reference) (OtherBodyIndex :type Integer) (bFromSweep :type Boolean) (SweepResult :type Hit%20Result%20Structure%20%28by%20ref%29))
  ;[1 1 1] XP
  (bind _asxpbas_classe_item (Utilities|Casting|CastToXPBasClasseItem OtherActor))
  (Default|Stop _asxpbas_classe_item)
  (Variables|XP|SetXP (+ (Variables|XP|GetXP) (Variables|/Game/Project/Items/XP/XPBasClasseItem.XPBasClasseItem_C|GetXpToAdd _asxpbas_classe_item)))
  (Actor|DestroyActor _asxpbas_classe_item))

(event OnComponentBeginOverlap(Damage)
  (params (OverlappedComponent :type Primitive%20Component%20Object%20Reference) (OtherActor :type Actor%20Object%20Reference) (OtherComp :type Primitive%20Component%20Object%20Reference) (OtherBodyIndex :type Integer) (bFromSweep :type Boolean) (SweepResult :type Hit%20Result%20Structure%20%28by%20ref%29))
  ;[1 1 1] Take Damage
)

(event OnComponentEndOverlap(Damage)
  (params (OverlappedComponent :type Primitive%20Component%20Object%20Reference) (OtherActor :type Actor%20Object%20Reference) (OtherComp :type Primitive%20Component%20Object%20Reference) (OtherBodyIndex :type Integer))
  ;[1 1 1] Take Damage
)

(event Custom|LoseLife
  (params (Damage :type Float%20%28single-precision%29))
  (Variables|Default|SetLife (- (Variables|Default|GetLife) Damage)))

(event Custom|TakeDamage
  ;[1 1 1] Take Damage
  (bind _asennemie_base_class (Utilities|Casting|CastToEnnemieBaseClass (stale OnComponentBeginOverlap(Damage) OtherActor))
    (:CastFailed
      (Utilities|Time|ClearandInvalidateTimerbyHandle (Variables|Default|GetTimerDamages)))))

(event EventTick
  (params (DeltaSeconds :type Float%20%28single-precision%29))
  ;[1 1 1] Tick
  (CallFunction|LifeBarSet)
  (CallFunction|WidgetLookRotation)
  (if (<= (Variables|Default|GetLife) 0.0)
    (Utilities|FlowControl|DoOnce false
      (:Completed
        (Utilities|Time|ClearandInvalidateTimerbyHandle (Variables|Default|GetTimerDamages))
        (Input|DisableInput (Pawn|GetController) 0)
        (bind _returnvalue (UserInterface|CreateWidget "/Game/Project/UI/WBP_GameOver.WBP_GameOver_C"))
        (UserInterface|Viewport|AddtoViewport _returnvalue 0)))))

(event EventBeginPlay
  ;[1 1 1] Begin Play
  (Variables|/Script/Engine.PlayerController|SetbShowMouseCursor (Game|GetPlayerController 0) false)
  (Components|Activation|Activate (Variables|Default|GetCamera1) false)
  (bind _returnvalue (UserInterface|CreateWidget "/Game/Project/UI/WBP_HUD.WBP_HUD_C"))
  (UserInterface|Viewport|AddtoViewport _returnvalue 0)
  (bind _returnvalue_2 (UserInterface|CreateWidget "/Game/Project/UI/WBP_PlayerHeatlh.WBP_PlayerHeatlh_C"))
  (Variables|Default|SetLifeHeadUp _returnvalue_2))

(event Input|MouseEvents|LeftMouseButton
  (params (Key :type Key%20Structure :default "None"))
  (:Pressed
    (Variables|Default|SetCanAttack true)
    (Utilities|FlowControl|Delay 2.0)
    (Variables|Default|SetCanAttack false)))

(fn ConstructionScript)

(fn SaveValue
  (bind _returnvalue (SaveGame|DoesSaveGameExist (Variables|Default|GetMySave)))
  (if _returnvalue
    (bind _returnvalue_2 (SaveGame|LoadGamefromSlot (Variables|Default|GetMySave)))
    (bind _output_get (Variables|Default|SetSaver _returnvalue_2))
    (bind _asmy_save (Utilities|Casting|CastToMySave _output_get))
    (SaveGame|SaveGametoSlot _asmy_save (Variables|Default|GetMySave))
    (return _asmy_save)
    (else
      (bind _returnvalue_3 (SaveGame|CreateSaveGameObject "/Game/Project/Gameplay/Management/MySave.MySave_C"))
      (bind _output_get_2 (Variables|Default|SetSaver _returnvalue_3))
      (bind _asmy_save_2 (Utilities|Casting|CastToMySave _output_get_2))
      (SaveGame|SaveGametoSlot _asmy_save_2 (Variables|Default|GetMySave))
      (return _asmy_save_2))))

(fn WidgetLookRotation
  (Transformation|SetWorldRotation (Variables|Default|GetWidget1) (Math|Rotator|FindLookatRotation (Transformation|GetWorldLocation (Variables|Character|GetMesh)) (Transformation|GetWorldLocation (Variables|Default|GetCamera1))) false false))

(fn LifeBarSet
  (bind _lifeheadup (Variables|Default|GetLifeHeadUp))
  (Variables|/Game/Project/UI/WBP_PlayerHeatlh.WBP_PlayerHeatlh_C|SetLife _lifeheadup (Variables|Default|GetLife))
  (Utilities|FlowControl|DoOnce false
    (:Completed
      (Variables|/Game/Project/UI/WBP_PlayerHeatlh.WBP_PlayerHeatlh_C|SetMaxLife _lifeheadup (Variables|Default|GetMaxLife)))))